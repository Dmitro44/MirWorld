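; 2D flipbook character that players select by clicking it or through UI events and that reports task status to the game mode.
; Tick picks run, idle or attack flipbooks from movement direction and working state; attack always uses the front view.
; Selection toggles, with a Ctrl/Shift check for multi-select, and shows a selection marker.
; Selection changes, hover info and task completion or failure reach the game mode through BP_ISelection.
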(event `self.ReceiveBeginPlay`
  ;[1 1 1] Character Info Setting
  (set `self.Character Info` (`KismetTextLibrary.Conv_StringToText` (`KismetStringLibrary.Concat_StrStr` "Персонаж " (`KismetStringLibrary.Conv_IntToString` (+ (`self.GetID`) 1))))))

(event `self.ReceiveTick`
  (params (DeltaSeconds :type "Float (single-precision)"))
  (bind _sprite (`self.Sprite`))
  (`|ExecutionSequence`
    (:`then_0`
      ;[1 1 1] Animations
      (bind _returnvalue (`self.GetDirection`))
      (if (> (`KismetMathLibrary.VSize` _returnvalue) 0.0)
        (bind _output_get (set `self.Is Front` (< (.x _returnvalue) 0.0)))
        (if _output_get
          (`PaperFlipbookComponent.SetFlipbook` _sprite "/Game/BPs/CharactersAndMobs/Character/Flipbooks/FB_Run_Front.FB_Run_Front")
          (else
            (`PaperFlipbookComponent.SetFlipbook` _sprite "/Game/BPs/CharactersAndMobs/Character/Flipbooks/FP_Run_Back.FP_Run_Back")))
        (elif (`self.IsWorking`)
          (`PaperFlipbookComponent.SetFlipbook` _sprite "/Game/BPs/CharactersAndMobs/Character/Flipbooks/FP_Attack_Front.FP_Attack_Front")
          (elif _output_get
            (`PaperFlipbookComponent.SetFlipbook` _sprite "/Game/BPs/CharactersAndMobs/Character/Flipbooks/FB_Idle_Front.FB_Idle_Front")
            (else
              (`PaperFlipbookComponent.SetFlipbook` _sprite "/Game/BPs/CharactersAndMobs/Character/Flipbooks/FP_Idle_Back.FP_Idle_Back"))))))))

(event `self.Plane.OnBeginCursorOver`
  (params (TouchedComponent :type "PrimitiveComponent Object Reference"))
  (bind _returnvalue (`GameplayStatics.GetGameMode`))
  ;[1 1 1] Checks if the interface is implemented
  (if (`KismetSystemLibrary.DoesImplementInterface` _returnvalue "/Game/BPs/GameMods/BP_ISelection.BP_ISelection_C")
    ;[1 1 1] Use the interface
    (message `/Game/BPs/GameMods/BP_ISelection.Update Cursor Info` _returnvalue (`self.Character Info`))))

(event `self.ReceiveActorOnClicked`
  (params (ButtonPressed :type "Key Structure"))
  ;[1 1 1] Un/Selection
  (`self.Selection Func` :!label _label))

(event `UI click`
  (goto _label))

(event `Get Selected`
  (bind _returnvalue (`GameplayStatics.GetGameMode`))
  ;[1 1 1] Un/Selection by UI
  (if (`KismetSystemLibrary.DoesImplementInterface` _returnvalue "/Game/BPs/GameMods/BP_ISelection.BP_ISelection_C")
    (message `/Game/BPs/GameMods/BP_ISelection.Add Selected Character` _returnvalue self)
    (set `self.Is Selected` true)
    (`SceneComponent.SetVisibility` (`self.Selection`) (`self.Is Selected`) false :!label _label_2)))

(event `Get Unselected`
  (bind _returnvalue (`GameplayStatics.GetGameMode`))
  ;[1 1 1] Un/Selection by UI
  (if (`KismetSystemLibrary.DoesImplementInterface` _returnvalue "/Game/BPs/GameMods/BP_ISelection.BP_ISelection_C")
    (message `/Game/BPs/GameMods/BP_ISelection.Unselect Character` _returnvalue self)
    (set `self.Is Selected` false)
    (goto _label_2)))

(event `self.ReportDoneTask`
  (bind _returnvalue (`GameplayStatics.GetGameMode`))
  (if (`KismetSystemLibrary.DoesImplementInterface` _returnvalue "/Game/BPs/GameMods/BP_ISelection.BP_ISelection_C") :!label _label_3
    (message `/Game/BPs/GameMods/BP_ITasks.Set Char Busyness` _returnvalue self false)))

(event `self.ReportImpossibleTask`
  (goto _label_3))

(fn `Selection Func`
  (locals (`Temp Bool` :type Boolean))
  (bind _returnvalue (`GameplayStatics.GetGameMode`))
  ;[1 1 1] Checks
  (bind _output_get (set `self.Is Selected` (not (`self.Is Selected`))))
  (set `local.Temp Bool` _output_get)
  (if (`KismetSystemLibrary.DoesImplementInterface` _returnvalue "/Game/BPs/GameMods/BP_ISelection.BP_ISelection_C")
    (if (`self.Ctrl/Shift`)
      (if (`local.Temp Bool`) :!label _label
        ;[1 1 1] Character update
        (set `self.Is Selected` true :!label _label_2)
        (message `/Game/BPs/GameMods/BP_ISelection.Add Selected Character` _returnvalue self)
        (else
          (set `self.Is Selected` false)
          (message `/Game/BPs/GameMods/BP_ISelection.Unselect Character` _returnvalue self)))
      (else
        (bind _amnt (message `/Game/BPs/GameMods/BP_ISelection.Get Char Amnt` _returnvalue))
        (message `/Game/BPs/GameMods/BP_ISelection.Clear Selected Characters` _returnvalue)
        (if (> _amnt 1)
          (goto _label_2)
          (else
            (goto _label)))))
    (`SceneComponent.SetVisibility` (`self.Selection`) (`self.Is Selected`) false)))

(fn `UserConstructionScript`)