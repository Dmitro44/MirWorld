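; BP_TreeRes is a clickable tree resource actor that varies its look and name by biome.
; On BeginPlay it picks one of two random sprites for the biome and sets a Russian label for forest, tundra or desert (default).
; Cursor-over and click events pass the label and wood image to BP_GamePlayUI, which is found and cached on first use.
; Selection on click is marked TODO.
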(event `self.ReceiveBeginPlay`
  (`|ExecutionSequence`
    (:`then_0`
      ;[1 1 1] Setting tree's sprites depending on the biome type
      (`PaperSpriteComponent.SetSprite` (`self.PaperSprite`) (`|GetArrayItem` (`self.Tree Sprites`) (+ (* (`self.GetBiomeType`) 2) (`KismetMathLibrary.RandomIntegerInRange` 0 1))))
      (switch `int` (`self.GetBiomeType`)
        (:`Default`
          (set `self.Tree String` "Дерево (пустыня)"))
        (:`0`
          (set `self.Tree String` "Дерево (лес)"))
        (:`1`
          (set `self.Tree String` "Дерево (тундра)"))))))

(event `self.PaperSprite.OnBeginCursorOver`
  (params (TouchedComponent :type "PrimitiveComponent Object Reference"))
  ;[1 1 1] Updating cursor info
  (bind _ui (`self.Get UI Ref`))
  (`/Game/BPs/Widgets/BP_GamePlayUI.Object Over Event` _ui (`self.Tree String`)))

(event `self.PaperSprite.OnClicked`
  (params (TouchedComponent :type "PrimitiveComponent Object Reference") (ButtonPressed :type "Key Structure"))
  ;[1 1 1] Set selection (TODO)
  (bind _ui (`self.Get UI Ref`))
  (`/Game/BPs/Widgets/BP_GamePlayUI.Resource Click Event` _ui "/Game/Assets/WoodResImage.WoodResImage"))

(fn `Get UI Ref`
  (returns (UI :type "/Game/BPs/Widgets/BP_GamePlayUI Object Reference"))
  (`/Engine/EditorBlueprintResources/StandardMacros.IsValid` (`self.UI`)
    (:`Is Valid`
      _)
    (:`Is Not Valid`
      ;[1 1 1] Get UI ref
      (bind _foundwidgets (`WidgetBlueprintLibrary.GetAllWidgetsOfClass` "/Game/BPs/Widgets/BP_GamePlayUI.BP_GamePlayUI_C"))
      (bind _output_get (set `self.UI` (`|GetArrayItem` _foundwidgets)))))
  (return _output_get))

(fn `UserConstructionScript`)