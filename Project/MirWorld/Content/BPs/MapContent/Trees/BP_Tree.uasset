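; BP_Tree is a tree map object that presents itself as a wood resource with a biome-dependent look.
; On BeginPlay it picks one of two random sprite variants for its biome by indexing TreeSprites, then sets the wood icon and a Russian label for forest, tundra or desert (the default).
; Hovering the sprite updates the cursor info, and clicking it calls SetSelectionTODO.
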(event `self.ReceiveBeginPlay`
  (`|ExecutionSequence`
    (:`then_0`
      ;[1 1 1] Setting tree's sprites depending on the biome type
      (`PaperSpriteComponent.SetSprite` (`self.PaperSprite`) (`|GetArrayItem` (`self.Tree Sprites`) (+ (* (`self.GetBiomeType`) 2) (`KismetMathLibrary.RandomIntegerInRange` 0 1)))))
    (:`then_1`
      ;[1 1 1] Setting cursor info text
      (switch `int` (`self.GetBiomeType`)
        (:`Default`
          (set `self.Res Info Text` "Дерево (пустыня)"))
        (:`0`
          (set `self.Res Info Text` "Дерево (лес)"))
        (:`1`
          (set `self.Res Info Text` "Дерево (тундра)")))
      (set `self.Res Image` "/Game/Assets/WoodResImage.WoodResImage"))))

(event `self.PaperSprite.OnBeginCursorOver`
  (params (TouchedComponent :type "PrimitiveComponent Object Reference"))
  ;[1 1 1] Setting UI Info
  (`self.Update Cursor Info`))

(event `self.PaperSprite.OnClicked`
  (params (TouchedComponent :type "PrimitiveComponent Object Reference") (ButtonPressed :type "Key Structure"))
  ;[1 1 1] Setting UI Info
  (`self.Set Selection TODO`))

(fn `UserConstructionScript`)