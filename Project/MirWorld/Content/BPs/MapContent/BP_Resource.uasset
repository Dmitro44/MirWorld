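; Map resource Blueprint that can be selected, flagged as having a task and described in the cursor info.
; Selection routes through the game mode's BP_ISelection interface: appending toggles this resource, while a plain select clears the list and keeps it selected if several were selected.
; Separate bounds components show selected and task states, and UpdateCursorInfo sends its info text to the game mode.
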(event `Event Unselect`
  ;[1 1 1] Updates selection bounds' visibility
  (`SceneComponent.SetVisibility` (`self.Selection Bounds`) false false)
  (set `self.Is Selected` false))

(event `Event Set Has Task`
  (params (`Has Task` :type Boolean))
  ;[1 1 1] Sets task bounds' visibility
  (`SceneComponent.SetVisibility` (`self.Task Bounds`) `Has Task` false))

(fn `Set Selection TODO`
  (params (`Is Apeending` :type Boolean))
  (locals (`Temp Boolen` :type Boolean))
  (bind _returnvalue (`GameplayStatics.GetGameMode`))
  (set `local.Temp Boolen` (`self.Is Selected`))
  ;[1 1 1] Check if Gamemode does implement required interface
  (if (`KismetSystemLibrary.DoesImplementInterface` _returnvalue "/Game/BPs/GameMods/BP_ISelection.BP_ISelection_C")
    ;[1 1 1] Handles with multiselection
    (if `Is Apeending`
      (if (`local.Temp Boolen`) :!label _label
        (`self.Event Unselect`)
        (message `/Game/BPs/GameMods/BP_ISelection.Unselect Res` _returnvalue self)
        (else
          (message `/Game/BPs/GameMods/BP_ISelection.Add Selected Res` _returnvalue self :!label _label_2)
          (set `self.Is Selected` true)
          ;[1 1 1] Sprite update
          (`SceneComponent.SetVisibility` (`self.Selection Bounds`) true false)))
      (else
        (bind _amnt (message `/Game/BPs/GameMods/BP_ISelection.Get Res Amnt` _returnvalue))
        (message `/Game/BPs/GameMods/BP_ISelection.Clear Selected Res` _returnvalue)
        (if (> _amnt 1)
          (goto _label_2)
          (else
            (goto _label)))))))

(fn `Update Cursor Info`
  (bind _returnvalue (`GameplayStatics.GetGameMode`))
  ;[1 1 1] Check if Gamemode does implement required interface
  (if (`KismetSystemLibrary.DoesImplementInterface` _returnvalue "/Game/BPs/GameMods/BP_ISelection.BP_ISelection_C")
    (message `/Game/BPs/GameMods/BP_ISelection.Update Cursor Info` _returnvalue (`self.Res Info Text`))))

(fn `UserConstructionScript`)