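; BP_StoneRes is a stone resource map object that shows a paper sprite and reports to the gameplay UI.
; On BeginPlay it picks one of six sprites at random and sets a Russian hover label by biome, with the desert fallback reading "tree".
; Hover sends the label and click sends the resource image to a lazily cached BP_GamePlayUI widget.
; Selection is marked TODO.
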(event `self.ReceiveBeginPlay`
  ;[1 1 1] Setting cursor info text, and random stone sprites depending on the biome
  (`PaperSpriteComponent.SetSprite` (`self.PaperSprite`) (`|GetArrayItem` (`self.Stone Sprites`) (`KismetMathLibrary.RandomIntegerInRange` 0 5)))
  (switch `int` (`self.GetBiomeType`)
    (:`Default`
      (set `self.Stone String` "Дерево (пустыня)"))
    (:`0`
      (set `self.Stone String` "Булыжник (лес)"))
    (:`1`
      (set `self.Stone String` "Булыжник (тундра)"))))

(event `self.PaperSprite.OnBeginCursorOver`
  (params (TouchedComponent :type "PrimitiveComponent Object Reference"))
  ;[1 1 1] Updating cursor info
  (bind _ui (`self.Get UI Ref`))
  (`/Game/BPs/Widgets/BP_GamePlayUI.Object Over Event` _ui (`self.Stone String`)))

(event `self.PaperSprite.OnClicked`
  (params (TouchedComponent :type "PrimitiveComponent Object Reference") (ButtonPressed :type "Key Structure"))
  ;[1 1 1] Set selection (TODO)
  (bind _ui (`self.Get UI Ref`))
  (`/Game/BPs/Widgets/BP_GamePlayUI.Resource Click Event` _ui "/Game/Assets/StoneResImage.StoneResImage"))

(fn `Get UI Ref`
  (returns (UI :type "/Game/BPs/Widgets/BP_GamePlayUI Object Reference"))
  (`/Engine/EditorBlueprintResources/StandardMacros.IsValid` (`self.UI`)
    (:`Is Valid`
      _)
    (:`Is Not Valid`
      ;[1 1 1] Get UI ref
      (bind _foundwidgets (`WidgetBlueprintLibrary.GetAllWidgetsOfClass` "/Game/BPs/Widgets/BP_GamePlayUI.BP_GamePlayUI_C"))
      (bind _output_get (set `self.UI` (`|GetArrayItem` _foundwidgets)))))
  (return _output_get))

(fn `UserConstructionScript`)