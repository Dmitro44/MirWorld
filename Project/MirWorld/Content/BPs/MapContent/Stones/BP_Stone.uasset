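; BP_Stone is a clickable cobblestone resource placed on the map, shown as a Paper2D sprite.
; On BeginPlay it picks a random stone sprite and sets its resource image and a Russian, biome-specific name for forest, tundra or desert.
; Hovering updates the cursor info.
; Clicking outside the player pawn's building mode calls SetSelectionTODO, passing whether Ctrl or Shift is held.
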(event `self.ReceiveBeginPlay`
  (`|ExecutionSequence`
    (:`then_0`
      ;[1 1 1] Setting cursor random stone sprites depending on the biome
      (`PaperSpriteComponent.SetSprite` (`self.PaperSprite_0`) (`|GetArrayItem` (`self.Stone Sprites`) (`KismetMathLibrary.RandomIntegerInRange` 0 5))))
    (:`then_1`
      ;[1 1 1] Setting cursor info text
      (switch `int` (`self.GetBiomeType`)
        (:`Default`
          (set `self.Res Info Text` "Булыжник (пустыня)"))
        (:`0`
          (set `self.Res Info Text` "Булыжник (лес)"))
        (:`1`
          (set `self.Res Info Text` "Булыжник (тундра)")))
      (set `self.Res Image` "/Game/Assets/StoneResImage.StoneResImage"))))

(event `self.PaperSprite_0.OnBeginCursorOver`
  (params (TouchedComponent :type "PrimitiveComponent Object Reference"))
  ;[1 1 1] Setting UI Info
  (`self.Update Cursor Info`))

(event `self.PaperSprite_0.OnClicked`
  (params (TouchedComponent :type "PrimitiveComponent Object Reference") (ButtonPressed :type "Key Structure"))
  (bind _returnvalue (`GameplayStatics.GetPlayerController` 0))
  ;[1 1 1] Setting UI Info
  (bind _returnvalue_2 (`GameplayStatics.GetActorOfClass` "/Game/BPs/BP_PlayerPawn.BP_PlayerPawn_C"))
  (if (not (`/Game/BPs/BP_PlayerPawn.bIsBuidingModeOn` _returnvalue_2))
    (`self.Set Selection TODO` (or (`PlayerController.IsInputKeyDown` _returnvalue "LeftControl") (`PlayerController.IsInputKeyDown` _returnvalue "LeftShift") (`PlayerController.IsInputKeyDown` _returnvalue "RightShift") (`PlayerController.IsInputKeyDown` _returnvalue "RightControl")))))

(fn `UserConstructionScript`)