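; BP_Food is a food resource actor on the map, shown as a 2D Paper sprite that supports hover info and click selection.
; On BeginPlay it picks a random food sprite and sets its resource image and Russian label by biome (forest, tundra, otherwise desert).
; Hover updates cursor info; clicks outside the player pawn's building mode call SetSelectionTODO, passing whether Ctrl or Shift is held.
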(event `self.ReceiveBeginPlay`
  (`|ExecutionSequence`
    (:`then_0`
      (`PaperSpriteComponent.SetSprite` (`self.PaperSprite_0`) (`|GetArrayItem` (`self.Food Sprites`) (`KismetMathLibrary.RandomIntegerInRange` 0 6))))
    (:`then_1`
      (switch `int` (`self.GetBiomeType`)
        (:`Default`
          (set `self.Res Info Text` "Еда (пустыня)"))
        (:`0`
          (set `self.Res Info Text` "Еда (лес)"))
        (:`1`
          (set `self.Res Info Text` "Еда (тундра)")))
      (set `self.Res Image` "/Game/Assets/FoodResImage.FoodResImage"))))

(event `self.PaperSprite_0.OnBeginCursorOver`
  (params (TouchedComponent :type "PrimitiveComponent Object Reference"))
  (`self.Update Cursor Info`))

(event `self.PaperSprite_0.OnClicked`
  (params (TouchedComponent :type "PrimitiveComponent Object Reference") (ButtonPressed :type "Key Structure"))
  (bind _returnvalue (`GameplayStatics.GetPlayerController` 0))
  (bind _returnvalue_2 (`GameplayStatics.GetActorOfClass` "/Game/BPs/BP_PlayerPawn.BP_PlayerPawn_C"))
  (if (not (`/Game/BPs/BP_PlayerPawn.bIsBuidingModeOn` _returnvalue_2))
    (`self.Set Selection TODO` (or (`PlayerController.IsInputKeyDown` _returnvalue "LeftControl") (`PlayerController.IsInputKeyDown` _returnvalue "LeftShift") (`PlayerController.IsInputKeyDown` _returnvalue "RightControl") (`PlayerController.IsInputKeyDown` _returnvalue "RightShift")))))

(fn `UserConstructionScript`
  (`parent.UserConstructionScript`))