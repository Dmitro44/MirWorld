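; BP_Tile is a map surface tile whose material and Russian info string (desert, forest or tundra) are set from its biome type on BeginPlay.
; On cursor hover it passes its location to BP_PlayerPawn while building mode is on and shows the info string in BP_GamePlayUI.
; On click it clears resource and character selections through the game mode's BP_ISelection interface, a step marked TODO.
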(event `self.ReceiveBeginPlay`
  ;[1 1 1] Setting the color and the info string depending on the biome type
  (`PrimitiveComponent.SetMaterial` (`self.StaticMeshComponent`) 0 (`|GetArrayItem` (`self.Colors`) (`self.GetBiomeType`)))
  (switch `int` (`self.GetBiomeType`)
    (:`Default`
      (set `self.Tile String` "Поверхность (пустыня)"))
    (:`0`
      (set `self.Tile String` "Поверхность (лес)"))
    (:`1`
      (set `self.Tile String` "Поверхность (тундра)"))))

(event `self.StaticMeshComponent.OnBeginCursorOver`
  (params (TouchedComponent :type "PrimitiveComponent Object Reference"))
  (`|ExecutionSequence`
    (:`then_0`
      (bind _returnvalue (`GameplayStatics.GetActorOfClass` "/Game/BPs/BP_PlayerPawn.BP_PlayerPawn_C"))
      (if (`/Game/BPs/BP_PlayerPawn.bIsBuidingModeOn` _returnvalue)
        (set `/Game/BPs/BP_PlayerPawn.CurrentCursorLocation` (`self.K2_GetActorLocation`) _returnvalue)))
    (:`then_1`
      ;[1 1 1] Updating cursor info
      (bind _foundwidgets (`WidgetBlueprintLibrary.GetAllWidgetsOfClass` "/Game/BPs/Widgets/BP_GamePlayUI.BP_GamePlayUI_C"))
      (`/Game/BPs/Widgets/BP_GamePlayUI.Object Over Event` (`|GetArrayItem` _foundwidgets) (`self.Tile String`)))))

(event `self.StaticMeshComponent.OnClicked`
  (params (TouchedComponent :type "PrimitiveComponent Object Reference") (ButtonPressed :type "Key Structure"))
  (bind _returnvalue (`GameplayStatics.GetGameMode`))
  ;[1 1 1] End selection (TODO)
  (if (`KismetSystemLibrary.DoesImplementInterface` _returnvalue "/Game/BPs/GameMods/BP_ISelection.BP_ISelection_C")
    (message `/Game/BPs/GameMods/BP_ISelection.Clear Selected Res` _returnvalue)
    (message `/Game/BPs/GameMods/BP_ISelection.Clear Selected Characters` _returnvalue)))

(fn `UserConstructionScript`)