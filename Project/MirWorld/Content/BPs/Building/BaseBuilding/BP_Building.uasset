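; BP_Building is a building actor with a placement preview and a sprite shown once it is added to the map.
; While unplaced, box overlaps with non-tile actors are counted, toggling CanBePlaced and the cube's possible/impossible material.
; Placetomap swaps the cube for the sprite with its initial texture; BecomeReady is an empty completion event.
; Hovering the sprite sends BuildInfoText to the GameMode through BP_ISelection.
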(event `self.ReceiveBeginPlay`
  ;[1 1 1] Init
  (`PaperSpriteComponent.SetSprite` (`self.Building Sprite`) (`self.Ready Texture`)))

(event `Place to map`
  ;[1 1 1] Called when building has been added to the map
  (`SceneComponent.SetVisibility` (`self.Building Cube`) false false)
  (`SceneComponent.SetVisibility` (`self.Building Sprite`) true false)
  (`PaperSpriteComponent.SetSprite` (`self.Building Sprite`) (`self.Initial Texture`)))

(event `self.Box.OnComponentBeginOverlap`
  (params (OverlappedComponent :type "PrimitiveComponent Object Reference") (OtherActor :type "Actor Object Reference") (OtherComp :type "PrimitiveComponent Object Reference") (OtherBodyIndex :type Integer) (bFromSweep :type Boolean) (SweepResult :type "HitResult Structure (by ref)"))
  ;[1 1 1] Checks if can be placed
  (if (not (`self.IsPlaced`))
    (cast `/Game/BPs/MapContent/Tiles/BP_Tile` OtherActor
      (:`CastFailed`
        (`/Engine/EditorBlueprintResources/StandardMacros.IncrementInt` (`self.Overlap Cnr`)
          (:`  `
            (`PrimitiveComponent.SetMaterial` (`self.Building Cube`) 0 "/Game/BPs/Building/BaseBuilding/M_ImPossible.M_ImPossible")
            (set `self.CanBePlaced` false)))))))

(event `self.Box.OnComponentEndOverlap`
  (params (OverlappedComponent :type "PrimitiveComponent Object Reference") (OtherActor :type "Actor Object Reference") (OtherComp :type "PrimitiveComponent Object Reference") (OtherBodyIndex :type Integer))
  (bind _overlap_cnr (`self.Overlap Cnr`))
  ;[1 1 1] Checks if can be placed
  (if (not (`self.IsPlaced`))
    (cast `/Game/BPs/MapContent/Tiles/BP_Tile` OtherActor
      (:`CastFailed`
        (`/Engine/EditorBlueprintResources/StandardMacros.DecrementInt` _overlap_cnr
          (:`  `
            (if (<= _overlap_cnr 0)
              (`PrimitiveComponent.SetMaterial` (`self.Building Cube`) 0 "/Game/BPs/Building/BaseBuilding/M_Possible.M_Possible")
              (set `self.CanBePlaced` true))))))))

(event `self.BecomeReady`
  ;[1 1 1] Called when building is done
)

(event `self.Building Sprite.OnBeginCursorOver`
  (params (TouchedComponent :type "PrimitiveComponent Object Reference"))
  (bind _returnvalue (`GameplayStatics.GetGameMode`))
  ;[1 1 1] Check if Gamemode does implement required interface
  (if (`KismetSystemLibrary.DoesImplementInterface` _returnvalue "/Game/BPs/GameMods/BP_ISelection.BP_ISelection_C")
    (message `/Game/BPs/GameMods/BP_ISelection.Update Cursor Info` _returnvalue (`self.Build info Text`))))

(fn `UserConstructionScript`)