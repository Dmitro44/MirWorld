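; Game mode for gameplay that owns the in-game HUD and handles victory, defeat and score updates.
; BeginPlay creates the BP_GamePlayUI widget, stores it and adds it to the viewport.
; UpdateScore finds the ScoreCntr_BP actor, reads its score and writes it into the widget's ScoreValue if the widget is valid.
; The victory and defeat events only print placeholder text.
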(event `self.ReceiveBeginPlay`
  ;[1 1 1] UI setting
  (bind _returnvalue (`|CreateWidget` "/Game/BPs/Widgets/BP_GamePlayUI.BP_GamePlayUI_C"))
  (bind _output_get (set `self.UI` _returnvalue))
  (`UserWidget.AddToViewport` _output_get 0))

(event `self.EndGame_Defeat`
  ;[1 1 1] End game
  (`KismetSystemLibrary.PrintText` "D" true true (struct :`G` 0.66 :`B` 1.0 :`A` 1.0) 10.0))

(event `self.EndGame_Victory`
  ;[1 1 1] End game
  (`KismetSystemLibrary.PrintText` "V" true true (struct :`G` 0.66 :`B` 1.0 :`A` 1.0) 10.0))

(event `self.UpdateScore`
  (bind _ui (`self.UI`))
  ;[1 1 1] Update ui score cntr
  (bind _returnvalue (`GameplayStatics.GetActorOfClass` "/Game/TestBPs/ScoreCntr_BP.ScoreCntr_BP_C"))
  (bind _returnvalue_2 (`ScoreCntr.GetScore` _returnvalue))
  (`/Engine/EditorBlueprintResources/StandardMacros.IsValid` _ui
    (:`Is Valid`
      (set `/Game/BPs/Widgets/BP_GamePlayUI.ScoreValue` _returnvalue_2 _ui))))

(fn `UserConstructionScript`)