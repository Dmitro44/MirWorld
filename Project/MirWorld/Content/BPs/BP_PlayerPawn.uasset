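; Player pawn that runs a building placement mode, starting a craft bench preview on a key press.
; StartBuilding spawns the actor with the M_Possible material, and Tick keeps it hovering above CurrentCursorLocation.
; Left click places it if CanBePlaced, then BlockTiles marks the surrounding 3x3 tiles impassable in BP_MapGenerate.
; X cancels placement by destroying the preview.
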(event `Key|F`
  (params (Key :type "Key Structure"))
  (:`Pressed`
    (`/Game/BPs/Building/BaseBuilding/BP_IBuilding.StartBuilding` "/Game/BPs/Building/CraftBench/BP_CraftBench.BP_CraftBench_C")))

(event `Key|LeftMouseButton`
  (params (Key :type "Key Structure"))
  (:`Pressed`
    (`self.PlaceBuilding`)))

(event `Key|X`
  (params (Key :type "Key Structure"))
  (:`Pressed`
    (`self.DeleteBuilding`)))

(event `self.ReceiveTick`
  (params (DeltaSeconds :type "Float (single-precision)"))
  ;[1 1 1] Moving Object until build
  (if (`self.bIsBuidingModeOn`)
    (`self.K2_SetActorLocation` (`self.ObjectToSpawn`) (+ (`self.CurrentCursorLocation`) (0.0 0.0 300.0)) false false)))

(event `/Game/BPs/Building/BaseBuilding/BP_IBuilding.PlaceBuilding`
  (bind _objecttospawn (`self.ObjectToSpawn`))
  ;[1 1 1] Place Building
  (if (`self.bIsBuidingModeOn`)
    (if (`/Game/BPs/Building/BaseBuilding/BP_Building.Can Be Placed` (`self.ObjectToSpawn`))
      (set `self.bIsBuidingModeOn` false)
      (set `/Game/BPs/Building/BaseBuilding/BP_Building.Is Placed` true _objecttospawn)
      (`/Game/BPs/Building/BaseBuilding/BP_Building.Place to map` _objecttospawn)
      (`self.BlockTiles`))))

(event `/Game/BPs/Building/BaseBuilding/BP_IBuilding.DeleteBuilding`
  ;[1 1 1] Delete Building
  (if (`self.bIsBuidingModeOn`)
    (set `self.bIsBuidingModeOn` false)
    (set `/Game/BPs/Building/BaseBuilding/BP_Building.Is Placed` true (`self.ObjectToSpawn`))
    (`self.K2_DestroyActor` (`self.ObjectToSpawn`))))

(fn `BlockTiles`
  (locals (dx :type Byte) (dy :type Byte))
  (bind _returnvalue (`GameplayStatics.GetActorOfClass` "/Game/BPs/BP_MapGenerate.BP_MapGenerate_C"))
  ;[1 1 1] Blocks 3x3 area
  (for _index (range -1 2)
    (for _index_2 (range -1 2)
      (`Generator.SetTileIsPassable` _returnvalue (+ (`self.CurrentCursorLocation`) (`KismetMathLibrary.MakeVector` (* _index 100) (* _index_2 100))) false))))

(fn `StartBuilding`
  (params (BuildingType :type "/Game/BPs/Building/BaseBuilding/BP_Building Class Reference"))
  (`KismetSystemLibrary.PrintString` "Hello")
  (if (not (`self.bIsBuidingModeOn`))
    (set `self.bIsBuidingModeOn` true)
    (bind _returnvalue (`|SpawnActorFromClass` BuildingType (`KismetMathLibrary.MakeTransform` (+ (`self.CurrentCursorLocation`) (0.0 0.0 50.0))) "Undefined" "MultiplyWithRoot" null null))
    (bind _output_get (set `self.ObjectToSpawn` _returnvalue))
    (`PrimitiveComponent.SetMaterial` (`BasicActor.StaticMeshComponent` _output_get) 0 "/Game/BPs/Building/BaseBuilding/M_Possible.M_Possible")))

(fn `UserConstructionScript`)