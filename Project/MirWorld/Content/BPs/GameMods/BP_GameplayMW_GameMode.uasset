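; Game mode for the MW gameplay level that creates the main gameplay UI, enables cursor interaction and applies the game instance's music volume.
; It tracks multi-selected resources, aggregating amount left, minability and a mixed-type label and icon, then pushes them to the UI.
; Deselection adjusts the totals or rebuilds the selection.
; It also relays score and hover info to the UI; victory and defeat only print placeholder text.
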(event `self.ReceiveBeginPlay`
  (`|ExecutionSequence`
    (:`then_0`
      ;[1 1 1] UI setting
      (bind _returnvalue (`|CreateWidget` "/Game/BPs/Widgets/BP_GamePlayUI.BP_GamePlayUI_C"))
      (bind _output_get (set `self.Main UI` _returnvalue))
      (`UserWidget.AddToViewport` _output_get 0)
      ;[1 1 1] Activate mouse cursor and events
      (bind _returnvalue_2 (`InputDeviceLibrary.GetPlayerControllerFromPlatformUser` (struct)))
      (set `PlayerController.bShowMouseCursor` true _returnvalue_2)
      (set `PlayerController.bEnableClickEvents` true _returnvalue_2)
      (set `PlayerController.bEnableMouseOverEvents` true _returnvalue_2))
    (:`then_1`
      ;[1 1 1] Music Settings
      (`self.Event Set Music Multiplier`))))

(event `self.EndGame_Defeat`
  ;[1 1 1] End game
  (`KismetSystemLibrary.PrintText` "D" true true (struct :`G` 0.66 :`B` 1.0 :`A` 1.0) 10.0))

(event `self.EndGame_Victory`
  ;[1 1 1] End game
  (`KismetSystemLibrary.PrintText` "V" true true (struct :`G` 0.66 :`B` 1.0 :`A` 1.0) 10.0))

(event `self.UpdateScore`
  (bind _main_ui (`self.Main UI`))
  ;[1 1 1] Update ui score cntr
  (bind _returnvalue (`GameplayStatics.GetActorOfClass` "/Game/BPs/ScoreCntr_BP.ScoreCntr_BP_C"))
  (bind _returnvalue_2 (`ScoreCntr.GetScore` _returnvalue))
  (`/Engine/EditorBlueprintResources/StandardMacros.IsValid` _main_ui
    (:`Is Valid`
      (set `/Game/BPs/Widgets/BP_GamePlayUI.Score Value` _returnvalue_2 _main_ui))))

(event `Event Set Music Multiplier`
  ;[1 1 1] Update music settings
  (bind _asbp_mir_world_instance (cast `/Game/BPs/BP_MirWorldInstance` (`GameplayStatics.GetGameInstance`)))
  (bind _outactors (`GameplayStatics.GetAllActorsOfClass` "/Script/Engine.AmbientSound"))
  (`AudioComponent.SetVolumeMultiplier` (`AmbientSound.AudioComponent` (`|GetArrayItem` _outactors)) (`/Game/BPs/BP_MirWorldInstance.MusicMultiplier` _asbp_mir_world_instance)))

(event `/Game/BPs/GameMods/BP_ISelection.Add Selected Res`
  (params (`Selected Res` :type "/Game/BPs/MapContent/BP_Resource Object Reference"))
  (bind _returnvalue (`KismetArrayLibrary.Array_Length` (`self.Selected Resources`)))
  (`|ExecutionSequence`
    (:`then_0`
      ;[1 1 1] If any Resource can be mined
      (`KismetArrayLibrary.Array_Add` (`self.Selected Resources`) `Selected Res`)
      (set `self.Can Be Mined Cntr` (+ (`self.Can Be Mined Cntr`) (`/Game/BPs/MapContent/BP_Resource.Can Be Mined` `Selected Res`))))
    (:`then_1`
      ;[1 1 1] Increases Res Cntr
      (set `self.Res Cntr` (+ (`Resource.GetResourceLeft` `Selected Res`) (`self.Res Cntr`))))
    (:`then_2`
      ;[1 1 1] Checks if different resources are selected
      (set `self.Are Different` (or (not (`KismetStringLibrary.EqualEqual_StrStr` (`KismetTextLibrary.Conv_TextToString` (`/Game/BPs/MapContent/BP_Resource.Res Info Text` (`|GetArrayItem` (`self.Selected Resources`)))) (`KismetTextLibrary.Conv_TextToString` (`/Game/BPs/MapContent/BP_Resource.Res Info Text` `Selected Res`)))) (`self.Are Different`))))
    (:`then_3`
      ;[1 1 1] For multiselection (sets text info and image)
      (set `self.Temp Image` (`/Game/BPs/MapContent/BP_Resource.Res Image` `Selected Res`))
      (if (`self.Are Different`)
        (set `self.Temp Text` "Разное")
        (set `self.Temp Image` "/Game/Assets/safeimagekit-pixel-art__19_.safeimagekit-pixel-art__19_")
        (else
          (set `self.Temp Text` (`/Game/BPs/MapContent/BP_Resource.Res Info Text` `Selected Res`))))
      (if (> _returnvalue 1)
        (set `self.Temp Text` (`KismetTextLibrary.Conv_StringToText` (`KismetStringLibrary.Concat_StrStr` (`KismetTextLibrary.Conv_TextToString` (`self.Temp Text`)) " x" (`KismetStringLibrary.Conv_IntToString` _returnvalue))))))
    (:`then_4`
      ;[1 1 1] UI Update
      (`/Game/BPs/Widgets/BP_GamePlayUI.Resource Click Event` (`self.Main UI`) (`self.Temp Image`) (`self.Res Cntr`) (`self.Temp Text`) (`KismetMathLibrary.Conv_IntToBool` (`self.Can Be Mined Cntr`))))))

(event `/Game/BPs/GameMods/BP_ISelection.Clear Selected Res`
  (`|ExecutionSequence`
    (:`then_0`
      ;[1 1 1] Clear Selections
      (for _array_element (`self.Selected Resources`)
        (`/Game/BPs/MapContent/BP_Resource.Event Unselect` _array_element))
      ;[1 1 1] No Selected Resources now
      (`KismetArrayLibrary.Array_Clear` (`self.Selected Resources`))
      (set `self.Can Be Mined Cntr` 0)
      (set `self.Are Different` false))
    (:`then_1`
      ;[1 1 1] Update UI
      (`/Game/BPs/Widgets/BP_GamePlayUI.Resource Vis Update Event` (`self.Main UI`) false)
      ;[1 1 1] Resets the counter
      (set `self.Res Cntr` 0))))

(event `/Game/BPs/GameMods/BP_ISelection.Unselect Res`
  (params (Res :type "/Game/BPs/MapContent/BP_Resource Object Reference"))
  (`self.Erase Res` Res))

(event `/Game/BPs/GameMods/BP_ISelection.Update Cursor Info`
  (params (`Object Info` :type Text))
  ;[1 1 1] Info about the object under the mouse cursor
  (`/Game/BPs/Widgets/BP_GamePlayUI.Object Over Event` (`self.Main UI`) `Object Info`))

(fn `Erase Res`
  (params (InputPin :type "/Game/BPs/MapContent/BP_Resource Object Reference"))
  (locals (`Temp Array` :type "Array of /Game/BPs/MapContent/BP_Resource Object Reference"))
  (bind _main_ui (`self.Main UI`))
  (bind _output (`|GetArrayItem` (`self.Selected Resources`)))
  ;[1 1 1] Removes from array
  (bind _returnvalue (`KismetArrayLibrary.Array_RemoveItem` (`self.Selected Resources`) InputPin))
  (if _returnvalue
    ;[1 1 1] If no res selected changes mode
    (if (`KismetMathLibrary.Conv_IntToBool` (`KismetArrayLibrary.Array_Length` (`self.Selected Resources`)))
      (`|ExecutionSequence`
        (:`then_0`
          ;[1 1 1] Updates Can be mined Cntr
          (set `self.Can Be Mined Cntr` (- (`self.Can Be Mined Cntr`) (`/Game/BPs/MapContent/BP_Resource.Can Be Mined` InputPin))))
        (:`then_1`
          ;[1 1 1] Updates Res Cntr
          (set `self.Res Cntr` (- (`self.Res Cntr`) (`Resource.GetResourceLeft` InputPin))))
        (:`then_2`
          ;[1 1 1] Checks if text update is required
          (if (> (`KismetArrayLibrary.Array_Length` (`self.Selected Resources`)) 1)
            ;[1 1 1] More than one resource left ()
            (bind _output_get (set `local.Temp Array` (`self.Selected Resources`)))
            (`/Game/BPs/GameMods/BP_ISelection.Clear Selected Res`)
            (for _array_element _output_get
              (`/Game/BPs/GameMods/BP_ISelection.Add Selected Res` _array_element)
              (set `/Game/BPs/MapContent/BP_Resource.Is Selected` true _array_element)
              (`SceneComponent.SetVisibility` (`/Game/BPs/MapContent/BP_Resource.Selection Bounds` _array_element) true false))
            (else
              ;[1 1 1] One resource left
              (`/Game/BPs/Widgets/BP_GamePlayUI.Resource Click Event` (`self.Main UI`) (`/Game/BPs/MapContent/BP_Resource.Res Image` _output) (`Resource.GetResourceLeft` _output) (`/Game/BPs/MapContent/BP_Resource.Res Info Text` _output) (`/Game/BPs/MapContent/BP_Resource.Can Be Mined` _output))))))
      (else
        (set `/Game/BPs/Widgets/BP_GamePlayUI.Resource Visibility` false _main_ui)
        (`/Game/BPs/Widgets/BP_GamePlayUI.Object Over Event` _main_ui (`/Game/BPs/Widgets/BP_GamePlayUI.CursorInfoText` _main_ui))))))

(fn `UserConstructionScript`)