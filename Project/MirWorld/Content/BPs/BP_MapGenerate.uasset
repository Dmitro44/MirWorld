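; BP_MapGenerate is the world generator actor, building a 50x50 map through BuildMap (not defined here) on BeginPlay.
; LoadMap rebuilds a saved world from game instance data, but its new-or-load branch is disconnected.
; It validates the arrays, spawns tiles, trees and stones with biome-specific Russian labels, then repositions existing characters by index.
; SpawnGolds follows the same parallel-array pattern, but LoadMap never calls it.
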(event `self.ReceiveBeginPlay`
  (`self.BuildMap` (2500.0 2500.0 0.0) 50 50))

(fn `CheckLength`
  (params (Trees :type "Array of Transform Structure") (Tiles :type "Array of Transform Structure") (Stones :type "Array of Transform Structure") (NewParam :type "Array of Transform Structure"))
  (returns (Correct :type Boolean))
  (return (and (> (`KismetArrayLibrary.Array_Length` Trees) 0) (> (`KismetArrayLibrary.Array_Length` Tiles) 0) (> (`KismetArrayLibrary.Array_Length` Stones) 0) (> (`KismetArrayLibrary.Array_Length` NewParam) 0))))

(fn `LoadMap`
  (bind _savedata (message `/Game/BPs/SaveGame/Interfaces/BPI_SaveGame.GetGameData` (`GameplayStatics.GetGameInstance`)))
  (bind (_trees_transform _trees_biome _trees_randnums _trees_resourseleft) (break `/Game/BPs/SaveGame/Structures/S_Trees` (`/Game/BPs/SaveGame/BP_SaveGame.Trees` _savedata)))
  (bind (_tiles_transform _tiles_material) (break `/Game/BPs/SaveGame/Structures/S_Tiles` (`/Game/BPs/SaveGame/BP_SaveGame.Tiles` _savedata)))
  (bind (_stones_transform _stones_biome _stones_randnum _stones_resourseleft) (break `/Game/BPs/SaveGame/Structures/S_Stone` (`/Game/BPs/SaveGame/BP_SaveGame.Stones` _savedata)))
  (bind (_players_transform _players_info) (break `/Game/BPs/SaveGame/Structures/S_PlayerSave` (`/Game/BPs/SaveGame/BP_SaveGame.Players` _savedata)))
  (bind _correct (`self.CheckLength` _trees_transform _tiles_transform _stones_transform _players_transform))
  (if _correct
    (`self.Spawn Tiles` _tiles_transform _tiles_material)
    (`self.Spawn Trees` _trees_transform _trees_biome _trees_randnums _trees_resourseleft)
    (`self.Spawn Stones` _stones_transform _stones_biome _stones_randnum _stones_resourseleft)
    (`self.Spawn Characters` _players_transform _players_info)))

(fn `Spawn Characters`
  (params (Transform :type "Array of Transform Structure") (Info :type "Array of Text"))
  (bind _outactors (`GameplayStatics.GetAllActorsOfClass` "/Game/BPs/CharactersAndMobs/BP_CharacterMW2D.BP_CharacterMW2D_C"))
  (for (_array_element _array_index) _outactors
    (`self.K2_SetActorTransform` _array_element (`|GetArrayItem` Transform _array_index) false true)
    (set `/Game/BPs/CharactersAndMobs/BP_CharacterMW2D.Character Info` (`|GetArrayItem` Info _array_index) _array_element)))

(fn `Spawn Golds`
  (params (Transform :type "Array of Transform Structure") (Biome :type "Array of Integer") (`Rand Num` :type "Array of Integer") (`Res Left` :type "Array of Integer"))
  (for (_array_element _array_index) Transform
    (bind _returnvalue (`|SpawnActorFromClass` "/Game/BPs/MapContent/Gold/BP_Gold.BP_Gold_C" _array_element "Undefined" "MultiplyWithRoot" null null))
    (`PaperSpriteComponent.SetSprite` (`/Game/BPs/MapContent/Gold/BP_Gold.PaperSprite_0` _returnvalue) (`|GetArrayItem` (`/Game/BPs/MapContent/Gold/BP_Gold.Gold Sprites` _returnvalue) (`|GetArrayItem` `Rand Num` _array_index)))
    (`Resource.SetResourceLeft` _returnvalue (`|GetArrayItem` `Res Left` _array_index))
    (switch `int` (`|GetArrayItem` Biome _array_index)
      (:`Default`
        (set `/Game/BPs/MapContent/BP_Resource.Res Info Text` "Золото (пустыня)" _returnvalue))
      (:`0`
        (set `/Game/BPs/MapContent/BP_Resource.Res Info Text` "Золото (лес)" _returnvalue))
      (:`1`
        (set `/Game/BPs/MapContent/BP_Resource.Res Info Text` "Золото (тундра)" _returnvalue)))))

(fn `Spawn Stones`
  (params (Transform :type "Array of Transform Structure") (Biome :type "Array of Integer") (RandNum :type "Array of Integer") (ResLeft :type "Array of Integer"))
  (for (_array_element _array_index) Transform
    (bind _returnvalue (`|SpawnActorFromClass` "/Game/BPs/MapContent/Stones/BP_Stone.BP_Stone_C" _array_element "Undefined" "MultiplyWithRoot" null null))
    ;[1 1 1] Bug with textures
    (`PaperSpriteComponent.SetSprite` (`/Game/BPs/MapContent/Stones/BP_Stone.PaperSprite_0` _returnvalue) (`|GetArrayItem` (`/Game/BPs/MapContent/Stones/BP_Stone.Stone Sprites` _returnvalue) (`|GetArrayItem` RandNum _array_index)))
    (`Resource.SetResourceLeft` _returnvalue (`|GetArrayItem` ResLeft _array_index))
    (switch `int` (`|GetArrayItem` Biome _array_index)
      (:`Default`
        (set `/Game/BPs/MapContent/BP_Resource.Res Info Text` "Булыжник (пустыня)" _returnvalue))
      (:`0`
        (set `/Game/BPs/MapContent/BP_Resource.Res Info Text` "Булыжник (лес)" _returnvalue))
      (:`1`
        (set `/Game/BPs/MapContent/BP_Resource.Res Info Text` "Булыжник (тундра)" _returnvalue)))))

(fn `Spawn Tiles`
  (params (Resources :type "Array of Transform Structure") (Biome :type "Array of Integer"))
  (for (_array_element _array_index) Resources
    (bind _returnvalue (`|SpawnActorFromClass` "/Game/BPs/MapContent/Tiles/BP_Tile.BP_Tile_C" (`KismetMathLibrary.MakeTransform` (.location _array_element) (.rotation _array_element)) "Undefined" "MultiplyWithRoot" null null))
    (bind _output (`|GetArrayItem` Biome _array_index))
    (`PrimitiveComponent.SetMaterial` (`BasicActor.StaticMeshComponent` _returnvalue) 0 (`|GetArrayItem` (`/Game/BPs/MapContent/Tiles/BP_Tile.Colors` _returnvalue) _output))
    (switch `int` _output
      (:`Default`
        (set `/Game/BPs/MapContent/Tiles/BP_Tile.Tile String` "Поверхность (пустыня)" _returnvalue))
      (:`0`
        (set `/Game/BPs/MapContent/Tiles/BP_Tile.Tile String` "Поверхность (лес)" _returnvalue))
      (:`1`
        (set `/Game/BPs/MapContent/Tiles/BP_Tile.Tile String` "Поверхность (тундра)" _returnvalue)))))

(fn `Spawn Trees`
  (params (Trees :type "Array of Transform Structure") (Biome :type "Array of Integer") (RandNum :type "Array of Integer") (ResLeft :type "Array of Integer"))
  (for (_array_element _array_index) Trees
    (bind _returnvalue (`|SpawnActorFromClass` "/Game/BPs/MapContent/Trees/BP_Tree.BP_Tree_C" _array_element "Undefined" "MultiplyWithRoot" null null))
    (bind _output (`|GetArrayItem` Biome _array_index))
    ;[1 1 1] Bug with textures
    (`PaperSpriteComponent.SetSprite` (`/Game/BPs/MapContent/Trees/BP_Tree.PaperSprite_0` _returnvalue) (`|GetArrayItem` (`/Game/BPs/MapContent/Trees/BP_Tree.Tree Sprites` _returnvalue) (+ (* _output 2) (`|GetArrayItem` RandNum _array_index))))
    (`Resource.SetResourceLeft` _returnvalue (`|GetArrayItem` ResLeft _array_index))
    (switch `int` _output
      (:`Default`
        (set `/Game/BPs/MapContent/BP_Resource.Res Info Text` "Дерево (пустыня)" _returnvalue))
      (:`0`
        (set `/Game/BPs/MapContent/BP_Resource.Res Info Text` "Дерево (лес)" _returnvalue))
      (:`1`
        (set `/Game/BPs/MapContent/BP_Resource.Res Info Text` "Дерево (тундра)" _returnvalue)))))

(fn `UserConstructionScript`)