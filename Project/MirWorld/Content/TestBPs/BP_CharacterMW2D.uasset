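; BP_CharacterMW2D is a 2D flipbook character that follows trajectories and shows run, attack or idle animations.
; BeginPlay sends it along a hardcoded waypoint path as a movement test.
; Tick picks a front or back flipbook from movement direction and working state, keeping the last facing in IsFront while stationary.
; An unconnected test snippet would increase the score on ScoreCntr_BP.
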(event `self.ReceiveBeginPlay`
  ;[1 1 1] movement test
  (`self.SetStartPos` (50.0 50.0 0.0))
  (bind _output_get (set `self.trajectory` (`|MakeArray` (50.0 150.0 0.0) (150.0 250.0 0.0) (250.0 250.0 0.0) (350.0 250.0 0.0) (350.0 350.0 0.0) (350.0 450.0 0.0) :!type "Vector Structure")))
  (`self.SetTrajectory` _output_get)
  (`self.FollowTrajectory`))

(event `self.ReceiveActorBeginOverlap`
  (params (OtherActor :type "Actor Object Reference")))

(event `self.ReceiveTick`
  (params (DeltaSeconds :type "Float (single-precision)"))
  (bind _sprite (`self.Sprite`))
  (`|ExecutionSequence`
    (:`then_0`
      ;[1 1 1] Animations
      (bind _returnvalue (`self.GetDirection`))
      (if (> (`KismetMathLibrary.VSize` _returnvalue) 0.0)
        (bind _output_get (set `self.IsFront` (< (.x _returnvalue) 0.0)))
        (if _output_get
          (`PaperFlipbookComponent.SetFlipbook` _sprite "/Game/TestBPs/Character/Flipbooks/FB_Run_Front.FB_Run_Front")
          (else
            (`PaperFlipbookComponent.SetFlipbook` _sprite "/Game/TestBPs/Character/Flipbooks/FP_Run_Back.FP_Run_Back")))
        (elif (`self.IsWorking`)
          (if _output_get
            (`PaperFlipbookComponent.SetFlipbook` _sprite "/Game/TestBPs/Character/Flipbooks/FP_Attack_Front.FP_Attack_Front")
            (else
              (`PaperFlipbookComponent.SetFlipbook` _sprite "/Game/TestBPs/Character/Flipbooks/FP_Attack_Back.FP_Attack_Back")))
          (elif _output_get
            (`PaperFlipbookComponent.SetFlipbook` _sprite "/Game/TestBPs/Character/Flipbooks/FB_Idle_Front.FB_Idle_Front")
            (else
              (`PaperFlipbookComponent.SetFlipbook` _sprite "/Game/TestBPs/Character/Flipbooks/FP_Idle_Back.FP_Idle_Back"))))))))

(fn `UserConstructionScript`)